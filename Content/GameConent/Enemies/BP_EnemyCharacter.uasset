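; Base enemy character that serves the AI attack and target interface, with the range check returning false.
; AC_Health damage drives red overlay flash, timed health bar, throttled hit reacts interrupting AI via blackboard, and target sharing with nearby enemies.
; Death sets the blackboard flag, adds score, feeds linked doors, optionally drops a key, then expires.
; Construction links child skeletal meshes to the main mesh's pose and creates their dynamic overlay materials.
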(event OnDamaged(AC_Health)
  (params (bDead :type Boolean) (Damage :type Float%20%28double-precision%29) (HitLocation :type Vector :default "0, 0, 0") (DamageCauser :type Actor%20Object%20Reference))
  ;[0.05 0.05 0.05] On Damage Taken
  (CallFunction|HandleDamage bDead DamageCauser))

(event Custom|RedFlash
  ;[0.05 0.05 0.05] Flash Overlay Materials
  (bind _alpha (Timeline|TL_FlashOnHit PlayFromStart)
    (:Update
      (for _array_element (Variables|Default|GetOverlayMatInstances)
        (Rendering|Material|SetScalarParameterValue _array_element "Alpha" _alpha :!class /Script/Engine.MaterialInstanceDynamic)))))

(event EventSaveComplete
  ;[0.05 0.05 0.05] Handle Checkpoint
  (Actor|DestroyActor))

(event EventEnemeySetEnemyTarget
  (params (Actor :type Actor%20Object%20Reference))
  ;[0.05 0.05 0.05] Set Target
  (Variables|Default|SetEnemyTarget Actor))

(fn ConstructionScript
  (CallFunction|SetAllChildSkeletalMeshes)
  (Components|SkinnedMesh|SetLeaderPoseComponent (Variables|Default|GetAllChildSkeletalMeshes) (Variables|Character|GetMesh) false false)
  (CallFunction|SetOverlayMaterials))

(fn SetOverlayMaterials
  (Utilities|Array|Clear (Variables|Default|GetOverlayMatInstances))
  (LocalVariables|SetLAllSkeletalMeshes (Variables|Default|GetAllChildSkeletalMeshes))
  (Utilities|Array|Add (LocalVariables|GetLAllSkeletalMeshes) (Variables|Character|GetMesh))
  (bind _overlaymaterial (Variables|Default|GetOverlayMaterial)
    (:then
      (for _array_element (LocalVariables|GetLAllSkeletalMeshes)
        (bind _returnvalue (Rendering|Material|CreateDynamicMaterialInstance _overlaymaterial "None" "None" :!class /Script/Engine.KismetMaterialLibrary))
        (Utilities|Array|Add (Variables|Default|GetOverlayMatInstances) _returnvalue)
        (Rendering|Material|SetOverlayMaterial _array_element _returnvalue :!class /Script/Engine.MeshComponent)))
    (:else)))

(fn UpdateHealthBar
  (bind _ac_health (Variables|Default|GetAC_Health))
  (bind _ac_health_2 (Variables|Default|GetAC_Health))
  (if (not (Rendering|IsVisible (Variables|Default|GetHealthWidget)))
    (Rendering|SetVisibility (Variables|Default|GetHealthWidget) true false)
    (bind _aswgt_enemy_health (Utilities|Casting|CastToWGT_EnemyHealth (UserInterface|GetWidget (Variables|Default|GetHealthWidget))))
    (bind _output_get (Variables|Default|SetEnemyHealthUI _aswgt_enemy_health))
    (Default|SetHealthPercent _output_get (Variables|/Game/GameConent/Core/AC_Health.AC_Health_C|GetHealth _ac_health) (Variables|/Game/GameConent/Core/AC_Health.AC_Health_C|GetMaxHealth _ac_health))
    (Utilities|Time|SetTimerbyFunctionName 0 "HideHealthUI" 1e+01)
    (else
      (bind _enemyhealthui (Variables|Default|GetEnemyHealthUI)
        (:then
          (Default|SetHealthPercent _enemyhealthui (Variables|/Game/GameConent/Core/AC_Health.AC_Health_C|GetHealth _ac_health_2) (Variables|/Game/GameConent/Core/AC_Health.AC_Health_C|GetMaxHealth _ac_health_2))
          (Utilities|Time|SetTimerbyFunctionName 0 "HideHealthUI" 1e+01))
        (:else)))))

(fn HideHealthUI
  (Rendering|SetVisibility (Variables|Default|GetHealthWidget) false false))

(fn PlayAttackAnimation
  (bind _attackanimation (Variables|Animations|GetAttackAnimation))
  (bind _returnvalue (Animation|Montage|MontagePlay (Components|SkeletalMesh|GetAnimInstance (Variables|Character|GetMesh)) (Utilities|Array|Get(acopy) _attackanimation (Math|Random|RandomIntegerinRange 0 (- (Utilities|Array|Length _attackanimation) 1))) 1.0 "Duration" 0.0 true))
  (return _returnvalue))

(fn SetTragetifNone
  (params (TargetActor :type Actor%20Object%20Reference))
  (Variables|Default|GetEnemyTarget
    (:then)
    (:else
      (bind _asbp_enemy_controller (Utilities|Casting|CastToBP_EnemyController (Pawn|GetController)))
      (Default|SetEnemyTarget _asbp_enemy_controller TargetActor))))

(fn OnDeath
  (params (DamageCauser :type Actor%20Object%20Reference))
  (CallFunction|FaceActor DamageCauser)
  (CallFunction|UpdateHealthBar)
  (Utilities|Time|SetTimerbyFunctionName 0 "HideHealthUI" 1.0)
  (CallFunction|SetCollisionstoDeath)
  (CallFunction|UnlockDoorifSet)
  (CallFunction|DropKeyifSet)
  (AI|Components|Blackboard|SetValueasBool (AI|GetBlackboard (Pawn|GetController)) (Utilities|Name|MakeLiteralName "bIsDead") true)
  (bind _asbp_game_instance (Utilities|Casting|CastToBP_GameInstance (Game|GetGameInstance)))
  (Default|AddEnemiesKilled _asbp_game_instance (Variables|Default|GetScoreValue))
  (Actor|SetLifeSpan 5.0))

(fn HandleDamage
  (params (bIsDead :type Boolean) (DamageCauser :type Actor%20Object%20Reference))
  (LocalVariables|SetLDamageCauser DamageCauser)
  (bind _output_get (Variables|Default|SetbIsDead bIsDead))
  (if _output_get
    (if (not (Variables|Default|GetbHasRunDeath))
      (CallFunction|RedFlash)
      (CallFunction|OnDeath (LocalVariables|GetLDamageCauser))
      (Variables|Default|SetbHasRunDeath true)
      (CallFunction|PlayTakeDamageAudio)
      (CallFunction|AlertNearbyEnemies))
    (else
      (CallFunction|SetTragetifNone (LocalVariables|GetLDamageCauser))
      (CallFunction|AlertNearbyEnemies)
      (CallFunction|RedFlash)
      (CallFunction|UpdateHealthBar)
      (CallFunction|HitReact (LocalVariables|GetLDamageCauser))
      (CallFunction|PlayTakeDamageAudio))))

(fn AllowHitReact
  (Variables|Default|SetbShouldPlayHitReact true))

(fn HitReact
  (params (DamageCauser :type Actor%20Object%20Reference))
  (bind _hitreactanimation (Variables|Animations|GetHitReactAnimation))
  (LocalVariables|SetLDamageCauser DamageCauser)
  (if (Variables|Default|GetbShouldPlayHitReact)
    (AI|Components|Blackboard|SetValueasBool (AI|GetBlackboard (Pawn|GetController)) (Utilities|Name|MakeLiteralName "bIsInterrupted") true)
    (bind _returnvalue (Animation|Montage|MontagePlay (Components|SkeletalMesh|GetAnimInstance (Variables|Character|GetMesh)) (Utilities|Array|Get(acopy) _hitreactanimation (Math|Random|RandomIntegerinRange 0 (- (Utilities|Array|Length _hitreactanimation) 1))) 1.0 "Duration" 0.0 true))
    (Variables|Default|SetbShouldPlayHitReact false)
    (Utilities|Time|SetTimerbyFunctionName 0 "AllowHitReact" (/ _returnvalue 2.0))
    (CallFunction|FaceActor (LocalVariables|GetLDamageCauser))))

(fn SetCollisionstoDeath
  (Collision|SetCollisionResponsetoAllChannels (Variables|Collision|GetCapsuleComponent) "ECR_Ignore")
  (Collision|SetCollisionResponsetoChannel (Variables|Collision|GetCapsuleComponent) "ECC_WorldStatic" "ECR_Block"))

(fn UnlockDoorifSet
  (for _array_element (Variables|OnDeath|GetDoorsToUnlock)
    (Utilities|IsValid _array_element
      (:Is%20Valid
        (Default|AddKey _array_element)))))

(fn AlertNearbyEnemies
  (bind _outactors (Collision|SphereOverlapActors (Transformation|GetActorLocation) (Variables|Enemy|GetAlertRange) (Utilities|Array|MakeArray "ObjectTypeQuery10") "BP_EnemyCharacter_C" (Utilities|Array|MakeArray self)))
  (for _array_element _outactors
    (bind _asbp_enemy_character (Utilities|Casting|CastToBP_EnemyCharacter _array_element))
    (CallFunction|SetTragetifNone _asbp_enemy_character (Variables|Default|GetEnemyTarget))))

(fn DropKeyifSet
  (if (Variables|OnDeath|GetbDropKey)
    (Game|SpawnActorfromClass "/Game/GameConent/GameplayMechanics/Collectables/Keys/BP_Col_SpecialKey.BP_Col_SpecialKey_C" (Math|Transform|MakeTransform (Transformation|GetWorldLocation (Variables|Default|GetEnemyGroundLoc)) "0, 0, 0" "1.000000,1.000000,1.000000") "Undefined" 0 (Variables|OnDeath|GetKeyTag) 0)))

(fn FaceActor
  (params (Actor :type Actor%20Object%20Reference))
  (bind _returnvalue (Transformation|GetActorRotation))
  (Utilities|IsValid Actor
    (:Is%20Valid
      (Transformation|SetActorRotation (Math|Rotator|MakeRotator (.roll _returnvalue) (.pitch _returnvalue) (.yaw (Math|Rotator|FindLookatRotation (Transformation|GetActorLocation) (Transformation|GetActorLocation Actor))))))))

(fn PlayTakeDamageAudio
  (Audio|PlaySoundatLocation (Variables|Default|GetDamageSound) (Transformation|GetActorLocation) "0, 0, 0" 1.0 1.0 0.0 0 0 0 0))

(fn SetAllChildSkeletalMeshes
  (Utilities|Array|Clear (Variables|Default|GetAllChildSkeletalMeshes))
  (for _array_element (Components|GetChildrenComponents (Variables|Character|GetMesh) false)
    (bind _asskeletal_mesh_component (Utilities|Casting|CastToSkeletalMeshComponent _array_element))
    (Utilities|Array|Add (Variables|Default|GetAllChildSkeletalMeshes) _asskeletal_mesh_component))
  (return))

(fn EnemyAttack
  (bind _duration (CallFunction|PlayAttackAnimation))
  (return _duration))

(fn EnemyCheckTargetinRange
  (params (Target :type Actor%20Object%20Reference))
  (return false))

(fn EnemyGetEnemyTarget
  (return (Variables|Default|GetEnemyTarget)))

(fn EnemyIsDead
  (return (Variables|/Game/GameConent/Core/AC_Health.AC_Health_C|GetbIsDead (Variables|Default|GetAC_Health))))