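; Ranged robot enemy that attacks by firing rifle projectiles, auto-aimed at its current target.
; On the EnemyDoDamage event, it rotates the projectile spawn point toward EnemyTarget, or resets its relative rotation when no valid target exists.
; It then spawns the projectile there regardless of collision, owned by the robot and carrying its Damage value.
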(event EventEnemyDoDamage
  ;[0.05 0.05 0.05] Fire Projectile and Auto Aim At Player
  (bind _enemytarget (Variables|Default|GetEnemyTarget)
    (:then
      (Transformation|SetWorldRotation (Variables|Default|GetProjSpawnLoc) (Math|Rotator|FindLookatRotation (Transformation|GetWorldLocation (Variables|Default|GetProjSpawnLoc)) (Transformation|GetActorLocation _enemytarget)) false false))
    (:else
      (Transformation|SetRelativeRotation (Variables|Default|GetProjSpawnLoc) "0, 0, 0" false false)))
  (Game|SpawnActorfromClass "/Game/GameConent/Weapons/Projectiles/Projectile_E_Rifle.Projectile_E_Rifle_C" (Transformation|GetWorldTransform (Variables|Default|GetProjSpawnLoc)) "AlwaysSpawn" self (Variables|Default|GetDamage) 0))

(fn ConstructionScript
  (|CallParentFunction))